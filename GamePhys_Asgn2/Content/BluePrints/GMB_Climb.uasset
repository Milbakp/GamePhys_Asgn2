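; Game mode for the Climb level, where the goal is to collect every TriggerOrb.
; BeginPlay counts the orbs, creates the level, pause and win widgets, and spawns one of three hinge-joint models at the pawn's location based on the game instance's ModelType.
; Tick toggles the pause UI and runs the timer from GameStateGMB.
; When no orbs remain, it shows the win UI, calls the velocity-reset dispatch and plays a victory sound once.
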(event `self.ReceiveBeginPlay`
  (bind _returnvalue (`GameplayStatics.GetPlayerController` 0))
  (bind (_returnvalue_location _returnvalue_rotation _returnvalue_scale) (`KismetMathLibrary.BreakTransform` (`self.GetTransform` (`GameplayStatics.GetPlayerPawn` 0))))
  (bind _returnvalue_2 (`KismetMathLibrary.MakeTransform` _returnvalue_location (struct :`Yaw` -90.0) _returnvalue_scale))
  ; Get number of orbs to be collected
  (bind _outactors (`GameplayStatics.GetAllActorsOfClass` "/Game/BluePrints/TriggerOrb.TriggerOrb_C"))
  (set `self.NumOfOrbs` (`KismetArrayLibrary.Array_Length` _outactors))
  (bind _returnvalue_3 (`|CreateWidget` "/Game/BluePrints/UI/LevelUI.LevelUI_C" _returnvalue))
  (bind _output_get (set `self.LevelUI` _returnvalue_3))
  (bind _returnvalue_4 (`|CreateWidget` "/Game/BluePrints/UI/Win_UI.Win_UI_C" _returnvalue))
  (bind _output_get_2 (set `self.WinUI` _returnvalue_4))
  (bind _returnvalue_5 (`|CreateWidget` "/Game/BluePrints/UI/Pause_UI.Pause_UI_C" _returnvalue))
  (bind _output_get_3 (set `self.PauseUI` _returnvalue_5))
  (`Widget.SetVisibility` _output_get_3 "Hidden")
  (`Widget.SetVisibility` _output_get_2 "Hidden")
  (`UserWidget.AddToViewport` _output_get 0)
  (`UserWidget.AddToViewport` _returnvalue_4 0)
  (`UserWidget.AddToViewport` _output_get_3 0)
  ; Spawn one of the 3 models, depending on the model type. Spawn location based on player pawn.
  (bind _assettings (cast `/Game/BluePrints/Menu/Settings` (`GameplayStatics.GetGameInstance`)))
  (bind _modeltype (`/Game/BluePrints/Menu/Settings.ModelType` _assettings))
  (if (`KismetStringLibrary.EqualEqual_StrStr` _modeltype "Human")
    (`|SpawnActorFromClass` "/Game/BluePrints/Joints/Hinge_Joint_BP.Hinge_Joint_BP_C" _returnvalue_2 "Undefined" "MultiplyWithRoot" null null)
    (elif (`KismetStringLibrary.EqualEqual_StrStr` _modeltype "Imbalance")
      (`|SpawnActorFromClass` "/Game/BluePrints/Joints/Imbalance_Hinge_Joint_BP.Imbalance_Hinge_Joint_BP_C" _returnvalue_2 "Undefined" "MultiplyWithRoot" null null)
      (else
        (`|SpawnActorFromClass` "/Game/BluePrints/Joints/YSnake_Hinge_Joint_BP_Child.YSnake_Hinge_Joint_BP_Child_C" _returnvalue_2 "Undefined" "MultiplyWithRoot" null null)))))

(event `self.ReceiveTick`
  (params (DeltaSeconds :type "Float (single-precision)"))
  (bind _pauseui (`self.PauseUI`))
  (bind _gamestategmb (`self.GameStateGMB`))
  ; Toggling Pause UI
  (if _gamestategmb
    (`Widget.SetVisibility` _pauseui "Hidden")
    (else
      (`Widget.SetVisibility` _pauseui "Visible")))
  (if (<= (`self.NumOfOrbs`) 0)
    ; Make win ui visible after collect all orbs and pausing the game
    (`Widget.SetVisibility` (`self.LevelUI`) "Hidden")
    (`Widget.SetVisibility` (`self.WinUI`) "Visible")
    (`self.ResetLinearVelDispatch`)
    (if (`self.PlaySoundOnce`)
      (`GameplayStatics.PlaySound2D` "/Game/Audio/eaglaxle-gaming-victory-464016.eaglaxle-gaming-victory-464016" 1.0 1.0 0.0 null null)
      (set `self.PlaySoundOnce` false))
    (elif _gamestategmb
      ; Game Timer
      (set `self.Timer` (+ (`GameplayStatics.GetWorldDeltaSeconds`) (`self.Timer`))))))

(fn `UserConstructionScript`)