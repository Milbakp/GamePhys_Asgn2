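; Player controller Blueprint that sets up mouse and Enhanced Input for what appears to be a climbing control scheme.
; BeginPlay shows the cursor, enables input and adds the IMC_CLIMB mapping context.
; Disconnected draft nodes would move a Hand_BP under the cursor to a deprojected mouse position with sweep, but they never run, nor do stray impulse and location nodes.
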(event `self.ReceiveBeginPlay`
  (bind _returnvalue (`GameplayStatics.GetPlayerController` 0))
  (set `self.bShowMouseCursor` true)
  (`self.EnableInput` _returnvalue)
  (message `EnhancedInputSubsystemInterface.AddMappingContext` (pcsubsystem `EnhancedInputLocalPlayerSubsystem` _returnvalue) "/Game/Input/IMC_CLIMB.IMC_CLIMB" 0 (struct)))

(fn `UserConstructionScript`)