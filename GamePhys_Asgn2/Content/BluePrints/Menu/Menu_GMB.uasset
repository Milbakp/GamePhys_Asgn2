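; Menu game mode Blueprint that sets up the main menu along with model select and level select screens.
; On BeginPlay it creates all three widgets for the first player controller, hides both select screens and adds all three to the viewport.
; ShowLevel, ShowModel and BackToMenu switch screens by only making the target widget visible, without hiding the others.
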(event `self.ReceiveBeginPlay`
  (bind _returnvalue (`GameplayStatics.GetPlayerController` 0))
  (bind _returnvalue_2 (`|CreateWidget` "/Game/BluePrints/Menu/Menu_Widget.Menu_Widget_C" _returnvalue))
  (bind _output_get (set `self.Menu` _returnvalue_2))
  (bind _returnvalue_3 (`|CreateWidget` "/Game/BluePrints/Menu/ModelSelect_Widget.ModelSelect_Widget_C" _returnvalue))
  (bind _output_get_2 (set `self.ModelSelect` _returnvalue_3))
  (bind _returnvalue_4 (`|CreateWidget` "/Game/BluePrints/Menu/LevelSelect_Widget.LevelSelect_Widget_C" _returnvalue))
  (bind _output_get_3 (set `self.LevelSelect` _returnvalue_4))
  (`Widget.SetVisibility` _output_get_3 "Hidden")
  (`Widget.SetVisibility` _output_get_2 "Hidden")
  (`UserWidget.AddToViewport` _output_get 0)
  (`UserWidget.AddToViewport` _output_get_2 0)
  (`UserWidget.AddToViewport` _output_get_3 0))

(fn `BackToMenu`
  (`Widget.SetVisibility` (`self.Menu`) "Visible"))

(fn `ShowLevel`
  (`Widget.SetVisibility` (`self.LevelSelect`) "Visible"))

(fn `ShowModel`
  (`Widget.SetVisibility` (`self.ModelSelect`) "Visible"))

(fn `UserConstructionScript`)