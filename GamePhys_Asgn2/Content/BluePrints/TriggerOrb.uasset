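; TriggerOrb is a red or blue orb that a Hinge_Joint_BP actor destroys with the matching hand, decrementing the GMB_Climb game mode's orb count.
; Every tick, random Y/Z impulses make the Sphere wander, and the collision component is teleported to follow it.
; On overlap, red requires the right hand and blue the left to be within a set distance of the actor's location, not the Sphere's.
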(event `self.ReceiveBeginPlay`
  (bind _sphere (`self.Sphere`))
  (if (`KismetStringLibrary.EqualEqual_StrStr` (`self.RedOrBlue`) "Red")
    (`PrimitiveComponent.SetMaterial` _sphere 0 "/Game/Material/Red.Red")
    (else
      (`PrimitiveComponent.SetMaterial` _sphere 0 "/Game/Material/Blue.Blue"))))

(event `self.ReceiveTick`
  (params (DeltaSeconds :type "Float (single-precision)"))
  (`SceneComponent.K2_SetWorldLocation` (`self.CollisionComponent`) (`SceneComponent.K2_GetComponentLocation` (`self.Sphere`)) false true)
  (`self.Wander`))

(event `self.ReceiveActorBeginOverlap`
  (params (OtherActor :type "Actor Object Reference"))
  (bind _ashinge_joint_bp (cast `/Game/BluePrints/Joints/Hinge_Joint_BP` OtherActor)
    (:`then`
      (if (`KismetStringLibrary.EqualEqual_StrStr` (`self.RedOrBlue`) "Red")
        (if (<= (`KismetMathLibrary.VSize` (- (`SceneComponent.K2_GetComponentLocation` (`/Game/BluePrints/Joints/Hinge_Joint_BP.RightHand` _ashinge_joint_bp)) (`self.K2_GetActorLocation`))) 200.0)
          (`KismetSystemLibrary.PrintString` "Destroy" :!label _label)
          (`self.K2_DestroyActor`)
          (bind _asgmb_climb (cast `/Game/BluePrints/GMB_Climb` (`GameplayStatics.GetGameMode`)))
          (set `/Game/BluePrints/GMB_Climb.NumOfOrbs` (- (`/Game/BluePrints/GMB_Climb.NumOfOrbs` _asgmb_climb) 1) _asgmb_climb))
        (elif (<= (`KismetMathLibrary.VSize` (- (`SceneComponent.K2_GetComponentLocation` (`/Game/BluePrints/Joints/Hinge_Joint_BP.LeftHand` _ashinge_joint_bp)) (`self.K2_GetActorLocation`))) 200.0)
          (goto _label))))
    (:`CastFailed`
      (`KismetSystemLibrary.PrintString` "Hello"))))

(fn `UserConstructionScript`)

(fn `Wander`
  (bind _sphere (`self.Sphere`))
  (if (`KismetSystemLibrary.IsValid` _sphere)
    (`PrimitiveComponent.AddImpulse` _sphere (* (`KismetMathLibrary.RandomUnitVector`) (0.0 500.0 500.0)) "None" false)))