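; Experimental physics climbing rig whose hands are pushed with the mouse under the climb game mode.
; The LeftHand input traces under the cursor and impulses whichever hand it hits toward that point, within a distance limit from Body.
; While GameState is on, Tick pins Body's velocity to zero, moves the player pawn to it and periodically samples hand positions for Punch detection.
; ResetLinearVelocity clears GameState and stops all static meshes.
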(event `self.ReceiveBeginPlay`
  (bind _returnvalue (`GameplayStatics.GetPlayerController` 0))
  (cast `/Game/BluePrints/GMB_Climb` (`GameplayStatics.GetGameMode`))
  (`self.EnableInput` _returnvalue)
  (message `EnhancedInputSubsystemInterface.AddMappingContext` (pcsubsystem `EnhancedInputLocalPlayerSubsystem` _returnvalue) "/Game/Input/IMC_CLIMB.IMC_CLIMB" 0 (struct))
  (bind _asgmb_climb (cast `/Game/BluePrints/GMB_Climb` (`GameplayStatics.GetGameMode`)))
  (add `/Game/BluePrints/GMB_Climb.ResetLinearVelDispatch` _asgmb_climb (`|CreateDelegate` :!event `ResetLinearVelocity`)))

(event `EnhancedInput|/Game/Input/RightHand`
  (params (ActionValue :type Boolean) (ElapsedSeconds :type "Float (double-precision)") (TriggeredSeconds :type "Float (double-precision)") (InputAction :type "InputAction Object Reference" :default "/Game/Input/RightHand.RightHand")))

(event `self.ReceiveTick`
  (params (DeltaSeconds :type "Float (single-precision)"))
  (if (`self.GameState`)
    (`PrimitiveComponent.SetPhysicsLinearVelocity` (`self.Body`) (0.0 0.0 0.0) false "None")
    (`self.K2_SetActorLocation` (`GameplayStatics.GetPlayerPawn` 0) (`SceneComponent.K2_GetComponentLocation` (`self.Body`)) false false)
    (bind _output_get (set `self.SetLocationTimer` (- (`self.SetLocationTimer`) (`GameplayStatics.GetWorldDeltaSeconds`))))
    (if (<= _output_get 0.0)
      (set `self.SetLocationTimer` 1.0)
      (set `self.RightPreviousLocation` (`SceneComponent.K2_GetComponentLocation` (`self.RightHand`)))
      (set `self.LeftPreviousLocation` (`SceneComponent.K2_GetComponentLocation` (`self.LeftHand`))))))

(event `EnhancedInput|/Game/Input/LeftHand`
  (params (ActionValue :type Boolean) (ElapsedSeconds :type "Float (double-precision)") (TriggeredSeconds :type "Float (double-precision)") (InputAction :type "InputAction Object Reference" :default "/Game/Input/LeftHand.LeftHand"))
  (bind _lefthand (`self.LeftHand`))
  (bind _righthand (`self.RightHand`))
  (bind _returnvalue (`SceneComponent.K2_GetComponentLocation` _lefthand))
  (bind _returnvalue_2 (`SceneComponent.K2_GetComponentLocation` _righthand))
  (bind (_bblockinghit _binitialoverlap _time _distance _location _impactpoint _normal _impactnormal _physmat _hitactor _hitcomponent) (`GameplayStatics.BreakHitResult` (`PlayerController.GetHitResultUnderCursorByChannel` (`GameplayStatics.GetPlayerController` 0) "TraceTypeQuery1" true)))
  (bind (_bblockinghit_2 _binitialoverlap_2 _time_2 _distance_2 _location_2 _impactpoint_2 _normal_2 _impactnormal_2 _physmat_2 _hitactor_2 _hitcomponent_2) (`GameplayStatics.BreakHitResult` (`PlayerController.GetHitResultUnderCursorByChannel` (`GameplayStatics.GetPlayerController` 0) "TraceTypeQuery1" true)))
  (bind _returnvalue_3 (== _hitcomponent_2 (`self.LeftHand`)))
  (bind _returnvalue_4 (== _hitcomponent _righthand))
  (:`Triggered`
    (if (`self.GameState`)
      (if _returnvalue_3
        (if (and _returnvalue_3 (<= (`KismetMathLibrary.VSize` (- (`SceneComponent.K2_GetComponentLocation` (`self.Body`)) _returnvalue)) 1000.0))
          (bind _output_get (set `self.LeftHandVector` (* (`KismetMathLibrary.Normal` (- _location_2 _returnvalue)) (`self.HandSpeed`))))
          (`PrimitiveComponent.AddImpulse` _lefthand _output_get "None" false)
          (`PrimitiveComponent.IgnoreActorWhenMoving` (`self.LeftHand`) (`ActorComponent.GetOwner` (`self.RightHand`)) true))
        (elif _returnvalue_4
          (if (and _returnvalue_4 (<= (`KismetMathLibrary.VSize` (- (`SceneComponent.K2_GetComponentLocation` (`self.Body`)) _returnvalue_2)) 1000.0))
            (bind _output_get_2 (set `self.RightHandVector` (* (`KismetMathLibrary.Normal` (- _location _returnvalue_2)) (`self.HandSpeed`))))
            (`PrimitiveComponent.AddImpulse` _righthand _output_get_2 "None" false)
            (`PrimitiveComponent.IgnoreActorWhenMoving` (`self.RightHand`) (`ActorComponent.GetOwner` (`self.LeftHand`)) true)))))))

(fn `Punch`
  (returns (PunchValid :type Boolean))
  (return (or (>= (`KismetMathLibrary.VSize` (- (`SceneComponent.K2_GetComponentLocation` (`self.LeftHand`)) (`self.LeftPreviousLocation`))) 250.0) (>= (`KismetMathLibrary.VSize` (- (`SceneComponent.K2_GetComponentLocation` (`self.RightHand`)) (`self.RightPreviousLocation`))) 250.0))))

(fn `ResetLinearVelocity`
  (set `self.GameState` false)
  (for _array_element (`self.K2_GetComponentsByClass` "/Script/Engine.StaticMeshComponent")
    (`PrimitiveComponent.SetPhysicsLinearVelocity` _array_element (0.0 0.0 0.0) false "None")))

(fn `UserConstructionScript`)