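; DummyMenuHinge is a physics dummy with a body and two hands, apparently a menu copy of a climbing character with its control logic disconnected.
; All events are empty; leftover unconnected graphs steer hands toward cursor hits, drive the body from hand velocities and bind to GMB_Climb.
; ResetLinearVelocity clears GameState and stops every static mesh.
; Punch reports whether either hand is far from its stored previous location.
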(event `self.ReceiveBeginPlay`)

(event `EnhancedInput|/Game/Input/RightHand`
  (params (ActionValue :type Boolean) (ElapsedSeconds :type "Float (double-precision)") (TriggeredSeconds :type "Float (double-precision)") (InputAction :type "InputAction Object Reference" :default "/Game/Input/RightHand.RightHand")))

(event `self.ReceiveTick`
  (params (DeltaSeconds :type "Float (single-precision)")))

(event `EnhancedInput|/Game/Input/LeftHand`
  (params (ActionValue :type Boolean) (ElapsedSeconds :type "Float (double-precision)") (TriggeredSeconds :type "Float (double-precision)") (InputAction :type "InputAction Object Reference" :default "/Game/Input/LeftHand.LeftHand")))

(fn `Punch`
  (returns (PunchValid :type Boolean))
  (return (or (>= (`KismetMathLibrary.VSize` (- (`SceneComponent.K2_GetComponentLocation` (`self.LeftHand`)) (`self.LeftPreviousLocation`))) 250.0) (>= (`KismetMathLibrary.VSize` (- (`SceneComponent.K2_GetComponentLocation` (`self.RightHand`)) (`self.RightPreviousLocation`))) 250.0))))

(fn `ResetLinearVelocity`
  (set `self.GameState` false)
  (for _array_element (`self.K2_GetComponentsByClass` "/Script/Engine.StaticMeshComponent")
    (`PrimitiveComponent.SetPhysicsLinearVelocity` _array_element (0.0 0.0 0.0) false "None")))

(fn `UserConstructionScript`)